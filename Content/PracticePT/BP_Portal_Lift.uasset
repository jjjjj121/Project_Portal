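; Puzzle lift that moves vertically, sideways or rolls in response to a laser receiver (LaserEnd) or pressed button (QuestButton).
; Paired events play or reverse separate timelines per trigger, with sound and material changes.
; Timelines mostly act as tick windows: each update adds a fixed delta, signed by trigger state, so travel depends on frame rate.
; Button rotation turns the Scene component with opposite sign, while laser rotation turns the root.
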(event Custom|Down%20Rotate%20Lift
  (Audio|PlaySoundatLocation "/Game/PracticePT/Widget/Sound/Lift_Down_SFX.Lift_Down_SFX" (Transformation|GetActorLocation) "0, 0, 0" 1.0 1.0 0.0 0 0 0)
  (Rendering|Material|SetMaterialbyName (Variables|Default|GetLift) "Color_BrightPink" "/Game/PracticePT/Material/Color_BrightPink.Color_BrightPink")
  (Rendering|Material|SetMaterialbyName (Variables|Default|GetLift) "Color_BrightPink" "/Game/PracticePT/Material/Color_BrightPink.Color_BrightPink")
  (Utilities|FlowControl|Sequence
    (:then_0
      (Utilities|IsValid (Variables|Default|GetLaser%20End)
        (:Is%20Valid
          (Timeline|Move%20Lift Reverse ; Laser
            (:Update
              (if (Variables|/Game/PracticePT/LaserTrapEnd.LaserTrapEnd_C|GetIs%20Receive%20Laser? (Variables|Default|GetLaser%20End))
                (Transformation|AddWorldRotation (Variables|Default|GetDefaultSceneRoot) (Math|Rotator|MakeRotator (Variables|Default|GetLiftUpRotateValue) 0.0 0.0) false false)
                (else
                  (Transformation|AddWorldRotation (Variables|Default|GetDefaultSceneRoot) (Math|Rotator|MakeRotator (* (Variables|Default|GetLiftUpRotateValue) -1.0) 0.0 0.0) false false))))))))
    (:then_1
      (Utilities|IsValid (Variables|Default|GetQuest%20Button)
        (:Is%20Valid
          (Timeline|타임라인_3 Reverse
            (:Update
              (if (Variables|/Game/PracticePT/QuestButton.QuestButton_C|GetIs%20Press%20Button? (Variables|Default|GetQuest%20Button))
                (Transformation|AddRelativeRotation (Variables|Default|GetScene) (Math|Rotator|MakeRotator (* (Variables|Default|GetLiftUpRotateValue) -1.0) 0.0 0.0) false false)
                (else
                  (Transformation|AddRelativeRotation (Variables|Default|GetScene) (Math|Rotator|MakeRotator (Variables|Default|GetLiftUpRotateValue) 0.0 0.0) false false))))))))))

(event Custom|Up%20Rotate%20Lift
  (Audio|PlaySoundatLocation "/Game/PracticePT/Widget/Sound/Lift_Up_SFX.Lift_Up_SFX" (Transformation|GetActorLocation) "0, 0, 0" 1.0 1.0 0.0 0 0 0)
  (Rendering|Material|SetMaterialbyName (Variables|Default|GetLift) "Color_BrightPink" "/Game/PracticePT/Material/Color_BrightPupple.Color_BrightPupple")
  (Rendering|Material|SetMaterialbyName (Variables|Default|GetLift) "Color_BrightPink" "/Game/PracticePT/Material/Color_BrightPupple.Color_BrightPupple")
  (Utilities|FlowControl|Sequence
    (:then_0
      (Utilities|IsValid (Variables|Default|GetLaser%20End)
        (:Is%20Valid
          (Timeline|Move%20Lift Play ; Laser
            (:Update
              (if (Variables|/Game/PracticePT/LaserTrapEnd.LaserTrapEnd_C|GetIs%20Receive%20Laser? (Variables|Default|GetLaser%20End))
                (Transformation|AddWorldRotation (Variables|Default|GetDefaultSceneRoot) (Math|Rotator|MakeRotator (Variables|Default|GetLiftUpRotateValue) 0.0 0.0) false false)
                (else
                  (Transformation|AddWorldRotation (Variables|Default|GetDefaultSceneRoot) (Math|Rotator|MakeRotator (* (Variables|Default|GetLiftUpRotateValue) -1.0) 0.0 0.0) false false))))))))
    (:then_1
      (Utilities|IsValid (Variables|Default|GetQuest%20Button)
        (:Is%20Valid
          (Timeline|타임라인_3 Play
            (:Update
              (if (Variables|/Game/PracticePT/QuestButton.QuestButton_C|GetIs%20Press%20Button? (Variables|Default|GetQuest%20Button))
                (Transformation|AddRelativeRotation (Variables|Default|GetScene) (Math|Rotator|MakeRotator (* (Variables|Default|GetLiftUpRotateValue) -1.0) 0.0 0.0) false false)
                (else
                  (Transformation|AddRelativeRotation (Variables|Default|GetScene) (Math|Rotator|MakeRotator (Variables|Default|GetLiftUpRotateValue) 0.0 0.0) false false))))))))))

(event Custom|Down%20Locate%20Lift
  (Audio|PlaySoundatLocation "/Game/PracticePT/Widget/Sound/Lift_Down_SFX.Lift_Down_SFX" (Transformation|GetActorLocation) "0, 0, 0" 1.0 1.0 0.0 0 0 0)
  (Rendering|Material|SetMaterialbyName (Variables|Default|GetLift) "Color_BrightPink" "/Game/PracticePT/Material/Color_BrightPink.Color_BrightPink")
  (Utilities|FlowControl|Sequence
    (:then_0
      (Utilities|IsValid (Variables|Default|GetLaser%20End)
        (:Is%20Valid
          (bind _새_트랙_0 (Timeline|타임라인_1 Reverse) ; Laser
            (:Update
              (if (Variables|/Game/PracticePT/LaserTrapEnd.LaserTrapEnd_C|GetIs%20Receive%20Laser? (Variables|Default|GetLaser%20End))
                (Transformation|AddRelativeLocation (Variables|Default|GetDefaultSceneRoot) (Math|Vector|MakeVector 0.0 0.0 (+ _새_트랙_0 (Variables|Default|GetLiftUpLocateValue))) false false)
                (else
                  (Transformation|AddRelativeLocation (Variables|Default|GetDefaultSceneRoot) (Math|Vector|MakeVector 0.0 0.0 (- _새_트랙_0 (Variables|Default|GetLiftUpLocateValue))) false false))))))))
    (:then_1
      (Utilities|IsValid (Variables|Default|GetQuest%20Button)
        (:Is%20Valid
          (Timeline|타임라인_2 Reverse ; Button
            (:Update
              (if (Variables|/Game/PracticePT/QuestButton.QuestButton_C|GetIs%20Press%20Button? (Variables|Default|GetQuest%20Button))
                (Transformation|AddRelativeLocation (Variables|Default|GetDefaultSceneRoot) (Math|Vector|MakeVector 0.0 0.0 (Variables|Default|GetLiftUpLocateValue)) false false)
                (else
                  (Transformation|AddRelativeLocation (Variables|Default|GetDefaultSceneRoot) (Math|Vector|MakeVector 0.0 0.0 (* (Variables|Default|GetLiftUpLocateValue) -1.0)) false false))))))))))

(event Custom|Left%20Lift
  (Audio|PlaySoundatLocation "/Game/PracticePT/Widget/Sound/Lift_Down_SFX.Lift_Down_SFX" (Transformation|GetActorLocation) "0, 0, 0" 1.0 1.0 0.0 0 0 0)
  (Utilities|FlowControl|Sequence
    (:then_0
      (Utilities|IsValid (Variables|Default|GetLaser%20End)
        (:Is%20Valid
          (Timeline|타임라인_0 Reverse ; laser
            (:Update
              (if (Variables|/Game/PracticePT/LaserTrapEnd.LaserTrapEnd_C|GetIs%20Receive%20Laser? (Variables|Default|GetLaser%20End))
                (Rendering|Material|SetMaterialbyName (Variables|Default|GetLift) "Color_BrightPink" "/Engine/MaterialTemplates/VertexAnimation/AdvancedFlag.AdvancedFlag")
                (Transformation|AddWorldOffset (Variables|Default|GetDefaultSceneRoot) (Math|Vector|MakeVector 0.0 (Variables|Default|GetLiftRightLocateValue) 0.0) false false)
                (else
                  (Rendering|Material|SetMaterialbyName (Variables|Default|GetLift) "Color_BrightPink" "/Game/PracticePT/Material/Color_BrightPink.Color_BrightPink")
                  (Transformation|AddWorldOffset (Variables|Default|GetDefaultSceneRoot) (Math|Vector|MakeVector 0.0 (* (Variables|Default|GetLiftRightLocateValue) -1.0) 0.0) false false))))))))
    (:then_1
      (Utilities|IsValid (Variables|Default|GetQuest%20Button)
        (:Is%20Valid
          (Timeline|타임라인_4 Reverse ; Button
            (:Update
              (if (Variables|/Game/PracticePT/QuestButton.QuestButton_C|GetIs%20Press%20Button? (Variables|Default|GetQuest%20Button))
                (Rendering|Material|SetMaterialbyName (Variables|Default|GetLift) "Color_BrightPink" "/Engine/MaterialTemplates/VertexAnimation/AdvancedFlag.AdvancedFlag")
                (Transformation|AddWorldOffset (Variables|Default|GetDefaultSceneRoot) (Math|Vector|MakeVector 0.0 (Variables|Default|GetLiftRightLocateValue) 0.0) false false)
                (else
                  (Rendering|Material|SetMaterialbyName (Variables|Default|GetLift) "Color_BrightPink" "/Game/PracticePT/Material/Color_BrightPink.Color_BrightPink")
                  (Transformation|AddWorldOffset (Variables|Default|GetDefaultSceneRoot) (Math|Vector|MakeVector 0.0 (* (Variables|Default|GetLiftRightLocateValue) -1.0) 0.0) false false))))))))))

(event Custom|Right%20Lift
  (Audio|PlaySoundatLocation "/Game/PracticePT/Widget/Sound/Lift_Up_SFX.Lift_Up_SFX" (Transformation|GetActorLocation) "0, 0, 0" 1.0 1.0 0.0 0 0 0)
  (Utilities|FlowControl|Sequence
    (:then_0
      (Utilities|IsValid (Variables|Default|GetLaser%20End)
        (:Is%20Valid
          (Timeline|타임라인_0 Play ; laser
            (:Update
              (if (Variables|/Game/PracticePT/LaserTrapEnd.LaserTrapEnd_C|GetIs%20Receive%20Laser? (Variables|Default|GetLaser%20End))
                (Rendering|Material|SetMaterialbyName (Variables|Default|GetLift) "Color_BrightPink" "/Engine/MaterialTemplates/VertexAnimation/AdvancedFlag.AdvancedFlag")
                (Transformation|AddWorldOffset (Variables|Default|GetDefaultSceneRoot) (Math|Vector|MakeVector 0.0 (Variables|Default|GetLiftRightLocateValue) 0.0) false false)
                (else
                  (Rendering|Material|SetMaterialbyName (Variables|Default|GetLift) "Color_BrightPink" "/Game/PracticePT/Material/Color_BrightPink.Color_BrightPink")
                  (Transformation|AddWorldOffset (Variables|Default|GetDefaultSceneRoot) (Math|Vector|MakeVector 0.0 (* (Variables|Default|GetLiftRightLocateValue) -1.0) 0.0) false false))))))))
    (:then_1
      (Utilities|IsValid (Variables|Default|GetQuest%20Button)
        (:Is%20Valid
          (Timeline|타임라인_4 Play ; Button
            (:Update
              (if (Variables|/Game/PracticePT/QuestButton.QuestButton_C|GetIs%20Press%20Button? (Variables|Default|GetQuest%20Button))
                (Rendering|Material|SetMaterialbyName (Variables|Default|GetLift) "Color_BrightPink" "/Engine/MaterialTemplates/VertexAnimation/AdvancedFlag.AdvancedFlag")
                (Transformation|AddWorldOffset (Variables|Default|GetDefaultSceneRoot) (Math|Vector|MakeVector 0.0 (Variables|Default|GetLiftRightLocateValue) 0.0) false false)
                (else
                  (Rendering|Material|SetMaterialbyName (Variables|Default|GetLift) "Color_BrightPink" "/Game/PracticePT/Material/Color_BrightPink.Color_BrightPink")
                  (Transformation|AddWorldOffset (Variables|Default|GetDefaultSceneRoot) (Math|Vector|MakeVector 0.0 (* (Variables|Default|GetLiftRightLocateValue) -1.0) 0.0) false false))))))))))

(event Custom|Up%20Locate%20Lift
  (Audio|PlaySoundatLocation "/Game/PracticePT/Widget/Sound/Lift_Up_SFX.Lift_Up_SFX" (Transformation|GetActorLocation) "0, 0, 0" 1.0 1.0 0.0 0 0 0)
  (Rendering|Material|SetMaterialbyName (Variables|Default|GetLift) "Color_BrightPink" "/Game/PracticePT/Material/Color_BrightPupple.Color_BrightPupple")
  (Utilities|FlowControl|Sequence
    (:then_0
      (Utilities|IsValid (Variables|Default|GetLaser%20End)
        (:Is%20Valid
          (bind _새_트랙_0 (Timeline|타임라인_1 Play) ; Laser
            (:Update
              (if (Variables|/Game/PracticePT/LaserTrapEnd.LaserTrapEnd_C|GetIs%20Receive%20Laser? (Variables|Default|GetLaser%20End))
                (Transformation|AddRelativeLocation (Variables|Default|GetDefaultSceneRoot) (Math|Vector|MakeVector 0.0 0.0 (+ _새_트랙_0 (Variables|Default|GetLiftUpLocateValue))) false false)
                (else
                  (Transformation|AddRelativeLocation (Variables|Default|GetDefaultSceneRoot) (Math|Vector|MakeVector 0.0 0.0 (- _새_트랙_0 (Variables|Default|GetLiftUpLocateValue))) false false))))))))
    (:then_1
      (Utilities|IsValid (Variables|Default|GetQuest%20Button)
        (:Is%20Valid
          (Timeline|타임라인_2 Play ; Button
            (:Update
              (if (Variables|/Game/PracticePT/QuestButton.QuestButton_C|GetIs%20Press%20Button? (Variables|Default|GetQuest%20Button))
                (Transformation|AddRelativeLocation (Variables|Default|GetDefaultSceneRoot) (Math|Vector|MakeVector 0.0 0.0 (Variables|Default|GetLiftUpLocateValue)) false false)
                (else
                  (Transformation|AddRelativeLocation (Variables|Default|GetDefaultSceneRoot) (Math|Vector|MakeVector 0.0 0.0 (* (Variables|Default|GetLiftUpLocateValue) -1.0)) false false))))))))))

(event EventBeginPlay)

(fn ConstructionScript
  (Variables|Default|SetLiftUpRotateValue (Variables|Default|GetLiftUpRotateValue))
  (Variables|Default|SetLiftRightLocateValue (Variables|Default|GetLiftRightLocateValue))
  (Variables|Default|SetLiftUpLocateValue (Variables|Default|GetLiftUpLocateValue)))